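; First-person player pawn for an item puzzle, handling movement, look, interaction and a timed on-screen message.
; Interact line-traces ahead and tries handlers in turn, matching pickups by name and the wardrobe by cast.
; Progress flags gate the sequence: crowbar breaks the barrel cover for gunpowder, which permits key pickup to open the wardrobe.
; A PhysicsHandle carries guns or swords at grab distance until Release or OnCrochetEnter drops them.
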(event `self.ReceiveBeginPlay`
  ;[1 1 1] Create Text UI
  (bind _returnvalue (`|CreateWidget` "/Game/BluePrint/UI.UI_C"))
  (bind _output_get (set `self.MainText` _returnvalue))
  (`UserWidget.AddToViewport` _output_get 0))

(event `InputAxis|Forward`
  (params (AxisValue :type "Float (single-precision)"))
  ;[1 1 1] Movement
  (`self.AddMovementInput` (* (`self.GetActorForwardVector` (`self.GetController`)) (1.0 1.0 0.0)) AxisValue))

(event `InputAxis|BackWard`
  (params (AxisValue :type "Float (single-precision)"))
  ;[1 1 1] Movement
  (`self.AddMovementInput` (* (`self.GetActorForwardVector` (`self.GetController`)) (1.0 1.0 0.0)) AxisValue))

(event `InputAction|Interact`
  (params (Key :type "Key Structure"))
  ;[1 1 1] Check if objects
  (:`Pressed`
    (bind _return_value (`self.GetCameraPosition`))
    (bind _return_value_2 (`self.GetCameraDistance`))
    (bind (_outhit _returnvalue) (`KismetSystemLibrary.LineTraceSingleForObjects` :`Start` _return_value :`End` _return_value_2 :`ObjectTypes` (`|MakeArray` "ObjectTypeQuery2" "ObjectTypeQuery4" :!type "EObjectTypeQuery Enum") :`DrawDebugType` "ForDuration"))
    ;[1 1 1] Handle Interaction
    (if _returnvalue
      (bind (_bblockinghit _binitialoverlap _time _distance _location _impactpoint _normal _impactnormal _physmat _hitactor _hitcomponent) (`GameplayStatics.BreakHitResult` _outhit))
      (bind _haspickedup (`self.PickUpCrowbar` _hitactor))
      (if (not _haspickedup)
        (bind _hasbrokeup (`self.BreakBarelCover` _hitactor))
        (if (not _hasbrokeup)
          (bind _haspickedup_2 (`self.PickUpKey` _hitactor))
          (if (not _haspickedup_2)
            (bind _hasopendoor (`self.TryOpenWardrobe` _hitactor))
            (if (not _hasopendoor)
              (`self.TryPickUpObjects` _hitactor _hitcomponent _location))))))))

(event `InputAxis|Left`
  (params (AxisValue :type "Float (single-precision)"))
  ;[1 1 1] Movement
  (`self.AddMovementInput` (* (`self.GetActorRightVector` (`self.GetController`)) (1.0 1.0 0.0)) AxisValue))

(event `InputAxis|Right`
  (params (AxisValue :type "Float (single-precision)"))
  ;[1 1 1] Movement
  (`self.AddMovementInput` (* (`self.GetActorRightVector` (`self.GetController`)) (1.0 1.0 0.0)) AxisValue))

(event `InputAxis|MouseX`
  (params (AxisValue :type "Float (single-precision)"))
  ;[1 1 1] Movement
  (`self.AddControllerYawInput` AxisValue))

(event `self.ReceiveTick`
  (params (DeltaSeconds :type "Float (single-precision)"))
  (bind _return_value (`self.GetCameraDistance`))
  (`PhysicsHandleComponent.SetTargetLocationAndRotation` (`self.PhysicsHandle`) _return_value (`self.GetControlRotation`)))

(event `InputAxis|MouseY`
  (params (AxisValue :type "Float (single-precision)"))
  ;[1 1 1] Movement
  (`self.AddControllerPitchInput` AxisValue))

(event `OnCrochetEnter`
  (if (`KismetSystemLibrary.IsValid` (`self.GrabbedActor`))
    (`PhysicsHandleComponent.ReleaseComponent` (`self.PhysicsHandle`))
    (set `self.GrabbedActor` null)))

(event `TextDisplayed`
  ;[1 1 1] Reset text
  (`KismetSystemLibrary.K2_ClearTimer` null "ClearText")
  (`KismetSystemLibrary.K2_SetTimer` null "ClearText" (`self.TextDisplayTime`)))

(event `InputAction|Release`
  (params (Key :type "Key Structure"))
  (:`Pressed`
    (`PhysicsHandleComponent.ReleaseComponent` (`self.PhysicsHandle`))
    (set `self.GrabbedActor` null)))

(fn `BreakBarelCover`
  (params (HitActor :type "Actor Object Reference"))
  (returns (HasBrokeUp :type Boolean))
  (locals (BreakUp :type Boolean))
  (if (`KismetStringLibrary.EqualEqual_StrStr` (`KismetSystemLibrary.GetObjectName` HitActor) "Couvercle")
    (if (`self.HasCrowbar`)
      (set `local.BreakUp` true)
      (set `self.HasPowder` true)
      (`self.K2_DestroyActor` HitActor)
      (`TextBlock.SetText` (`/Game/BluePrint/UI.MainText` (`self.MainText`)) "Acquired : Gun Powder")
      (`self.TextDisplayed`)))
  (return (`local.BreakUp`)))

(fn `ClearText`
  (`TextBlock.SetText` (`/Game/BluePrint/UI.MainText` (`self.MainText`)) "")
  (return))

(fn `GetCameraDistance`
  (returns (`Return value` :type "Vector Structure"))
  (bind _return_value (`self.GetCameraPosition`))
  (return (+ _return_value (* (`self.GetActorForwardVector` (`self.GetController`)) (`self.GrabDistance`)))))

(fn `GetCameraPosition`
  (returns (`Return value` :type "Vector Structure"))
  (return (+ (`self.K2_GetActorLocation`) (`KismetMathLibrary.MakeVector` 0.0 0.0 (`self.BaseEyeHeight`)))))

(fn `PickUpCrowbar`
  (params (HitActor :type "Actor Object Reference"))
  (returns (HasPickedUp :type Boolean))
  (locals (HasPickUp :type Boolean))
  (if (`KismetStringLibrary.EqualEqual_StrStr` (`KismetSystemLibrary.GetObjectName` HitActor) "crowbar")
    (set `self.HasCrowbar` true)
    (set `local.HasPickUp` true)
    (`self.K2_DestroyActor` HitActor)
    (`TextBlock.SetText` (`/Game/BluePrint/UI.MainText` (`self.MainText`)) "Acquired : Crowbar")
    (`self.TextDisplayed`)
    (else
      (set `local.HasPickUp` false)))
  (return (`local.HasPickUp`)))

(fn `PickUpKey`
  (params (HitActor :type "Actor Object Reference"))
  (returns (HasPickedUp :type Boolean))
  (locals (HasPicked :type Boolean))
  (if (`KismetStringLibrary.EqualEqual_StrStr` (`KismetSystemLibrary.GetDisplayName` HitActor) "key")
    (if (`self.HasPowder`)
      (set `local.HasPicked` true)
      (set `self.HasKey` true)
      (`TextBlock.SetText` (`/Game/BluePrint/UI.MainText` (`self.MainText`)) "Acquired : Wardrobe key")
      (`self.TextDisplayed`)
      (`self.K2_DestroyActor` HitActor)))
  (return (`local.HasPicked`)))

(fn `TryOpenWardrobe`
  (params (HitActor :type "Actor Object Reference"))
  (returns (HasOpenDoor :type Boolean))
  (locals (HasOpen :type Boolean))
  (bind _asbp_wardrobe (cast `/Game/BluePrint/BP_wardrobe` HitActor)
    (:`then`
      (if (`self.HasKey`)
        (`/Game/BluePrint/BP_wardrobe.OpenDoor` _asbp_wardrobe)
        (set `self.WardrobeIsOpen` true)
        (set `local.HasOpen` true)
        (else
          (`TextBlock.SetText` (`/Game/BluePrint/UI.MainText` (`self.MainText`)) "It is locked")
          (`self.TextDisplayed`))))
    (:`CastFailed`
      _))
  (return (`local.HasOpen`)))

(fn `TryPickUpObjects`
  (params (HitActor :type "Actor Object Reference") (HitComponent :type "PrimitiveComponent Object Reference") (Position :type "Vector Structure"))
  (if (not (`KismetSystemLibrary.IsValid` (`self.GrabbedActor`)))
    (cast `/Game/BluePrint/BP_gun` HitActor
      (:`then`
        _)
      (:`CastFailed`
        (cast `/Game/BluePrint/BP_sword` HitActor)))
    (`PrimitiveComponent.SetSimulatePhysics` HitComponent true)
    (`KismetSystemLibrary.PrintString` "Hello")
    (`PhysicsHandleComponent.GrabComponentAtLocation` (`self.PhysicsHandle`) HitComponent "None" Position)
    (set `self.GrabbedActor` HitActor)
    (return)))

(fn `UserConstructionScript`)