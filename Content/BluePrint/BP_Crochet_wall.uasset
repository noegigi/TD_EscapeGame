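; BP_Crochet_wall is a wall hook ("crochet") that snaps objects entering its trigger into place and reports them to the game mode.
; On begin overlap it calls OnCrochetEnter on MainPawn, moves the overlapping actor to its own location and rotation, and disables that component's physics.
; It then passes the actor and its Order to MainGameMode's OnObjectTrigger.
; On end overlap it sends only the Order, with no actor.
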(event `self.Trigger.OnComponentBeginOverlap`
  (params (OverlappedComponent :type "PrimitiveComponent Object Reference") (OtherActor :type "Actor Object Reference") (OtherComp :type "PrimitiveComponent Object Reference") (OtherBodyIndex :type Integer) (bFromSweep :type Boolean) (SweepResult :type "HitResult Structure (by ref)"))
  (bind (_returnvalue_location _returnvalue_rotation) (`KismetMathLibrary.BreakTransform` (`self.GetTransform`)))
  (bind _asmain_pawn (cast `/Game/BluePrint/MainPawn` (`GameplayStatics.GetPlayerPawn` 0)))
  (`/Game/BluePrint/MainPawn.OnCrochetEnter` _asmain_pawn)
  (`self.K2_SetActorLocationAndRotation` OtherActor _returnvalue_location _returnvalue_rotation false false)
  (`PrimitiveComponent.SetSimulatePhysics` OtherComp false)
  (bind _asmain_game_mode (cast `/Game/MainGameMode` (`GameplayStatics.GetGameMode`)))
  (`/Game/MainGameMode.OnObjectTrigger` _asmain_game_mode OtherActor (`self.Order`)))

(event `self.Trigger.OnComponentEndOverlap`
  (params (OverlappedComponent :type "PrimitiveComponent Object Reference") (OtherActor :type "Actor Object Reference") (OtherComp :type "PrimitiveComponent Object Reference") (OtherBodyIndex :type Integer))
  (bind _asmain_game_mode (cast `/Game/MainGameMode` (`GameplayStatics.GetGameMode`)))
  (`/Game/MainGameMode.OnObjectTrigger` _asmain_game_mode null (`self.Order`)))

(fn `UserConstructionScript`)